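; Forklift actor that drives in a loop along an indexed BP_Spline while simulating a lidar scan of its surroundings.
; Tick advances distance by speed, easing the transform halfway toward the spline point with a sideways offset.
; A half-second timer fires 50 random debug-drawn traces in a hemisphere opposite its forward vector.
; Hits on "NotPointCloud"-tagged actors refresh Points and accumulate in LidarPoints, whose clear is never run.
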(event `self.ReceiveBeginPlay`
  (if (>= (`self.SplineIndex`) 0)
    (bind _outactors (`GameplayStatics.GetAllActorsOfClass` "/Game/Forklift/Blueprints/BP_Spline.BP_Spline_C"))
    (set `self.Spline` (`/Game/Forklift/Blueprints/BP_Spline.Spline` (`|GetArrayItem` _outactors (`self.SplineIndex`)))))
  (`KismetSystemLibrary.K2_SetTimer` null "Traces" 0.5 true))

(event `Traces`
  (bind _returnvalue (`SceneComponent.K2_GetComponentLocation` (`self.Forklift`)))
  (bind (_x _y _z) (`KismetMathLibrary.BreakVector3f` _returnvalue))
  (`KismetArrayLibrary.Array_Clear` (`self.Points`))
  (for _ (range 1 51)
    (bind _outhit (`KismetSystemLibrary.LineTraceSingle` :`Start` (`KismetMathLibrary.MakeVector` _x _y (+ _z 200.0)) :`End` (+ _returnvalue (* (`KismetMathLibrary.RandomUnitVectorInConeInDegrees` (* (`SceneComponent.GetForwardVector` (`self.Forklift`)) -1.0) 90.0) 1000.0)) :`TraceChannel` "TraceTypeQuery1" :`DrawDebugType` "ForDuration" :`DrawTime` 1.0))
    (bind (_bblockinghit _binitialoverlap _time _distance _location _impactpoint _normal _impactnormal _physmat _hitactor) (`GameplayStatics.BreakHitResult` _outhit))
    (`/Engine/EditorBlueprintResources/StandardMacros.IsValid` _hitactor
      (:`Is Valid`
        (bind _output_get (set `self.isNotPointCloud` (`self.ActorHasTag` _hitactor "NotPointCloud")))
        (if _output_get
          (`KismetArrayLibrary.Array_Add` (`self.Points`) _location)
          (set `self.Location` (+ _location _normal))
          (`KismetArrayLibrary.Array_Add` (`self.LidarPoints`) (make `LidarPointCloudPoint` (`self.Location`) (`self.Color`) (`LidarPointCloudBlueprintLibrary.Conv_VectorToLidarPointCloudNormal` (`KismetMathLibrary.MakeVector` (.x _impactnormal) (.y _impactnormal))))))))))

(event `self.ReceiveTick`
  (params (DeltaSeconds :type "Float (single-precision)"))
  (bind _returnvalue (`SplineComponent.GetSplineLength` (`self.Spline`)))
  (bind _returnvalue_2 (+ (* DeltaSeconds (`self.Speed`)) (`self.Distance`)))
  (if (>= (`self.SplineIndex`) 0)
    (bind _output_get (set `self.Distance` (`KismetMathLibrary.SelectFloat` (- _returnvalue_2 _returnvalue) _returnvalue_2 (> (`self.Distance`) _returnvalue))))
    (`self.Move` _output_get)))

(event `Move`
  (params (Distance :type "Float (single-precision)"))
  (bind _spline (`self.Spline`))
  (bind (_result_location _result_rotation _result_scale) (`KismetMathLibrary.BreakTransform` (`|EaseFunction` "Linear" 0.5 (`SceneComponent.K2_GetComponentToWorld` (`self.Forklift`)) (`KismetMathLibrary.MakeTransform` (`SplineComponent.GetLocationAtDistanceAlongSpline` _spline Distance "World") (`SplineComponent.GetRotationAtDistanceAlongSpline` _spline Distance "Local") (0.5 0.5 0.5)))))
  (`SceneComponent.K2_SetWorldTransform` (`self.Forklift`) (`KismetMathLibrary.MakeTransform` (+ (* (`SplineComponent.FindRightVectorClosestToWorldLocation` (`self.Spline`) _result_location "Local") (`self.Offset`)) _result_location) _result_rotation _result_scale) false false))

(fn `UserConstructionScript`)