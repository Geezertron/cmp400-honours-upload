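; BP_PointCloud is an actor that merges lidar points from all BP_NPC2 actors into one live point cloud.
; On BeginPlay it clears existing cloud collision, caches those actors and starts two looping timers.
; A fast timer replaces the cloud's data with every NPC's LidarPoints2.
; A slower timer shifts the actor one unit along X, then rebuilds the cloud's collision.
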(event `self.ReceiveBeginPlay`
  (`|ExecutionSequence`
    (:`then_0`
      (`LidarPointCloud.RemoveCollision` (`LidarPointCloudComponent.PointCloud` (`self.LidarPointCloud`))))
    (:`then_1`
      (bind _outactors (`GameplayStatics.GetAllActorsOfClass` "/Game/Forklift/Character/BP_NPC2.BP_NPC2_C"))
      (set `self.Actors` _outactors)
      (`KismetSystemLibrary.K2_SetTimer` null "CollectPoints" 0.1 true))
    (:`then_2`
      (`KismetSystemLibrary.K2_SetTimer` null "BuildCollision" 2.0 true))))

(event `OnEndPlay_Event` :!signature `self.OnEndPlay`
  (params (Actor :type "Actor Object Reference") (EndPlayReason :type "EEndPlayReason Enum" :default "Destroyed")))

(event `BuildCollision`
  (`self.K2_SetActorLocation` (+ (`self.K2_GetActorLocation`) (1.0 0.0 0.0)))
  (`LidarPointCloud.BuildCollision` (`LidarPointCloudComponent.PointCloud` (`self.LidarPointCloud`))))

(event `CollectPoints`
  (`KismetArrayLibrary.Array_Clear` (`self.CloudPoints`))
  (for _array_element (`self.Actors`)
    (`KismetArrayLibrary.Array_Append` (`self.CloudPoints`) (`/Game/Forklift/Character/BP_NPC2.LidarPoints2` _array_element)))
  (`LidarPointCloud.SetData` (`LidarPointCloudComponent.GetPointCloud` (`self.LidarPointCloud`)) (`self.CloudPoints`)))

(fn `UserConstructionScript`)