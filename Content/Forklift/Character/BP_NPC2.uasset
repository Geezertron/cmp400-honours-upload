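; BP_NPC2 is an NPC that acts as a simulated LiDAR scanner, sampling surrounding geometry as point cloud data.
; A looping half-second timer fires hundreds of random visibility traces from above the mesh across a forward hemisphere, ignoring PointCloudTag actors.
; Hits on NotPointCloud-tagged actors refill Points each scan and accumulate in LidarPoints2 as normal-offset points with horizontally flattened normals.
; This graph only collects the points; it does not render them.
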(event `self.ReceiveBeginPlay`
  (bind _outactors (`GameplayStatics.GetAllActorsWithTag` "PointCloudTag"))
  (`KismetSystemLibrary.K2_SetTimer` null "Traces2" 0.5 true))

(event `Traces2`
  (bind _returnvalue (`SceneComponent.K2_GetComponentLocation` (`self.Mesh`)))
  (bind (_x _y _z) (`KismetMathLibrary.BreakVector3f` _returnvalue))
  (`KismetArrayLibrary.Array_Clear` (`self.Points`))
  (for _ (range 1 301)
    (bind _outhit (`KismetSystemLibrary.LineTraceSingle` (`KismetMathLibrary.MakeVector` _x _y (+ _z 175.0)) (+ _returnvalue (* (`KismetMathLibrary.RandomUnitVectorInConeInDegrees` (`SceneComponent.GetForwardVector` (`self.CapsuleComponent`)) 90.0) 5000)) "TraceTypeQuery1" false (stale `self.ReceiveBeginPlay` _outactors)))
    (bind (_bblockinghit _binitialoverlap _time _distance _location _impactpoint _normal _impactnormal _physmat _hitactor) (`GameplayStatics.BreakHitResult` _outhit))
    (`/Engine/EditorBlueprintResources/StandardMacros.IsValid` _hitactor
      (:`Is Valid`
        (bind _output_get (set `self.isNotPointCloud` (`self.ActorHasTag` _hitactor "NotPointCloud")))
        (if _output_get
          (`KismetArrayLibrary.Array_Add` (`self.Points`) _location)
          (set `self.Location` (+ _location _normal))
          (`KismetArrayLibrary.Array_Add` (`self.LidarPoints2`) (make `LidarPointCloudPoint` (`self.Location`) (struct :`B` 255 :`G` 255 :`R` 255 :`A` 255) (`LidarPointCloudBlueprintLibrary.Conv_VectorToLidarPointCloudNormal` (`KismetMathLibrary.MakeVector` (.x _impactnormal) (.y _impactnormal))))))))))

(fn `UserConstructionScript`)